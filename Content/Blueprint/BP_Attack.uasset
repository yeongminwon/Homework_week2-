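; BP_Attack is an actor Blueprint that computes an attack value from its Strength variable and prints a rating.
; On BeginPlay it converts Strength to an integer and passes it to CalculateAttack, which applies a linear multiply-and-add formula.
; A non-negative result prints a strong attack message and a negative one prints weak, so any non-negative Strength counts as strong.
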(event `self.ReceiveBeginPlay`
  (bind _attackvalue (`self.calculateAttack` (`KismetMathLibrary.Conv_Int64ToInt` (`self.Strength`))))
  (if (>= _attackvalue 0)
    (`KismetSystemLibrary.PrintString` "Strong Attack")
    (else
      (`KismetSystemLibrary.PrintString` "Weak"))))

(fn `calculateAttack`
  (params (StrengthVlue :type Integer))
  (returns (AttackValue :type Integer))
  (return (+ (* StrengthVlue 5) 10)))

(fn `UserConstructionScript`)